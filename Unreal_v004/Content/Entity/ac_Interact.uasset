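; Actor component that makes its owning entity interactable as a pickup, usable, breakable, save point or stock.
; InteractFunction receives player distance and input, and within range updates the HUD crosshair by entity type.
; On interaction, pickups message the owner to loot and despawn, while the other types send an interact call.
; Those types then get cleared to None by DelayedReEnabling, which restores them after a delay unless re-enabling is disabled.
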(event Custom|DelayedReEnabling
  (params (NeverReEnable :type Boolean) (ReEnableAfter :type Float%20%28single-precision%29))
  (Variables|Default|SetEntity_Type_Storage (Variables|Default|GetEntity_Type))
  (Variables|Default|SetEntity_Type "NewEnumerator4")
  (if (not NeverReEnable)
    (Utilities|FlowControl|Delay ReEnableAfter)
    (Variables|Default|SetEntity_Type (Variables|Default|GetEntity_Type_Storage))
    (Development|PrintString "RESET MODE")))

(event EventBeginPlay)

(event EventTick
  (params (DeltaSeconds :type Float%20%28single-precision%29)))

(fn InteractFunction
  (params (DistanceToPlayer :type Float%20%28single-precision%29) (HasPlayerInteracted :type Boolean) (HUD :type Game%20HUD%20Object%20Reference) (NeverReEnable :type Boolean) (ReEnableAfter :type Float%20%28single-precision%29))
  (if (Variables|Default|GetEnablePickup)
    (if (< DistanceToPlayer (+ (Variables|Default|GetInteract_Distance_Offset) (Variables|Default|GetInteract_Distance)))
      (Default|SetCrosshairDisplay HUD "NewEnumerator0" "" (Variables|Default|GetEntity_Type))
      (switch Utilities|FlowControl|Switch|Switchonenum_Entity_Type (Variables|Default|GetEntity_Type)
        (:NewEnumerator4)
        (:NewEnumerator0
          (if HasPlayerInteracted
            (Class|AcLootInterface|LootEvent(Message) (Components|GetOwner))
            (Class|AcRespawnDataInterface|EntityDespawnEvent(Message) (Components|GetOwner) true false)))
        (:NewEnumerator1)
        (:NewEnumerator2
          (if HasPlayerInteracted :!label _label
            (Class|AcInteractInterface|InteractCall(Message) (Components|GetOwner))
            (CallFunction|DelayedReEnabling NeverReEnable ReEnableAfter)))
        (:NewEnumerator3
          (goto _label))
        (:NewEnumerator5
          (goto _label))
        (:NewEnumerator6
          (goto _label))))))

(fn SetCrosshairDisplayjunk
  (params (Crosshair%20Enum :type HUD_crossHairEnum%20Enum :default "NewEnumerator0") (Crosshair%20Info :type String) (HUD :type Game%20HUD%20Object%20Reference))
  (Variables|/Game/HUD/GameHUD.GameHUD_C|SetCrosshair%20Enum HUD Crosshair%20Enum)
  (Variables|/Game/HUD/GameHUD.GameHUD_C|SetCrosshair%20Info HUD Crosshair%20Info))