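; Loot component that rolls up to three configured item drops for its owning entity and grants them to an inventory.
; LootFunction passes each slot's name, type and chance to DetermineLootDrop, which makes a percentage roll.
; Successful rolls look up the item database and add a random amount within the item's pickup range.
; Spawnable world loot is only a stub, and the logged amount is rolled separately from the granted one.
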(event EventBeginPlay)

(event EventTick
  (params (DeltaSeconds :type Float%20%28single-precision%29)))

(fn DetermineLootDrop
  (params (ID_Name :type Name) (Type :type enum_ItemType%20Enum :default "NewEnumerator0") (Chance :type Integer) (SpawnableLoot :type Boolean))
  (Development|PrintString (Utilities|String|Append (Utilities|String|ToString(Name) ID_Name) (Utilities|String|EnumtoString Type) (Utilities|String|ToString(Integer) Chance) (Utilities|String|ToString(Boolean) SpawnableLoot)))
  (if (< Chance (Math|Random|RandomIntegerinRange 1 100))
    _
    (else
      (bind _ac_itemdatabase (CallFunction|FuncGetItemDatabase))
      (bind (_display_name _item) (Default|GetItemInfo _ac_itemdatabase ID_Name Type))
      (CallFunction|FuncPrintErrorMessage (Utilities|String|Append "Item added to inventory: " (Utilities|String|ToString(Name) _display_name) ", Amount: " (Utilities|String|ToString(Integer) (Math|Random|RandomIntegerinRange (.PickupAmountMin (Utilities|Struct|Breaksuperstruct_Item _item)) (.PickupAmountMax (Utilities|Struct|Breaksuperstruct_Item _item))))) "NewEnumerator0" (Components|GetOwner) self (Variables|Default|GetPrint))
      (if SpawnableLoot
        (CallFunction|FuncPrintErrorMessage "No spawnable loot function implemented yet." "NewEnumerator1" (Components|GetOwner) self true)
        (else
          (bind _ac_inventory (CallFunction|FuncGetInventory))
          (Default|AddItemtoInventory _ac_inventory (Utilities|Struct|Makestruct_InventoryAdd ID_Name Type (Math|Random|RandomIntegerinRange (.PickupAmountMin (Utilities|Struct|Breaksuperstruct_Item _item)) (.PickupAmountMax (Utilities|Struct|Breaksuperstruct_Item _item)))))))))
  (return))

(fn LootFunction
  (CallFunction|DetermineLootDrop (Variables|Default|GetDrop1_ID_Name) (Variables|Default|GetDrop_1_Type) (Variables|Default|GetDrop_1_Chance) false)
  (CallFunction|DetermineLootDrop (Variables|Default|GetDrop2_ID_Name) (Variables|Default|GetDrop_2_Type) (Variables|Default|GetDrop_2_Chance) false)
  (CallFunction|DetermineLootDrop (Variables|Default|GetDrop3_ID_Name) (Variables|Default|GetDrop_3_Type) (Variables|Default|GetDrop_3_Chance) false))