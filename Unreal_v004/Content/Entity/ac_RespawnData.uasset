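; Actor component that remembers whether its owning entity is despawned, as either respawnable or permanent.
; It hides the owner at construction, then on BeginPlay registers with its Level Master HI for an ID from coordinates plus array index (respawnable) or offset manual ID (permanent).
; After a short delay, GameState's despawned lists decide whether the owner gets a spawn or despawn message.
; DespawnEntityFunction updates those lists, saves the game and messages the owner.
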(event Custom|Event_RespawnDataConstruction
  ;[0.9095 0 1] Dev Only : The only reason this Delay is required is for the thumbnail of each blueprint to not be empty.
  (if (Class|KismetSystemLibrary|IsPackagedforDistribution)
    _
    (else
      (Utilities|FlowControl|Delay 0.001)))
  (Rendering|SetActorHiddenInGame (Components|GetOwner) true)
  (CallFunction|CreateID false))

(event EventBeginPlay
  (bind _returnvalue (Components|GetOwner))
  (bind _respawnid (Variables|Default|GetRespawnID))
  (CallFunction|CreateID true)
  (Utilities|FlowControl|Delay 0.2)
  ;[1 1 1] superswitch
  (bind (_success _game_state) (CallFunction|FuncGetGameState))
  (if (Variables|Default|GetRespawnable)
    (Variables|Default|SetSpawn (== (Utilities|Array|FindItem (Variables|/Game/Blueprints/NewGameStateBase.NewGameStateBase_C|GetDespawnedEntities_Respawnable_IDs _game_state) _respawnid) -1))
    (else
      (Variables|Default|SetSpawn (== (Utilities|Array|FindItem (Variables|/Game/Blueprints/NewGameStateBase.NewGameStateBase_C|GetDespawnedEntities_Permanent_IDs _game_state) _respawnid) -1))))
  (if (Variables|Default|GetSpawn)
    (Rendering|SetActorHiddenInGame _returnvalue false)
    (Class|AcRespawnDataInterface|EntitySpawnCall(Message) _returnvalue false)
    (else
      (Class|AcRespawnDataInterface|EntityDespawnCall(Message) (Components|GetOwner) false false))))

(event EventTick
  (params (DeltaSeconds :type Float%20%28single-precision%29)))

(fn CreateID
  (params (SaveArrayToMasterNode :type Boolean))
  (bind _returnvalue (Components|GetOwner))
  (bind _returnvalue_2 (Components|GetOwner))
  (bind _returnvalue_3 (Components|GetOwner))
  (bind _id (Variables|Default|GetID))
  (Utilities|IsValid (Variables|Default|GetMaster_HI_reference)
    (:Is%20Valid
      (if SaveArrayToMasterNode
        (if (Variables|Default|GetRespawnable)
          (bind _returnvalue_4 (Utilities|Array|Add (Variables|/Game/World_Management/Level_Master_HI.Level_Master_HI_C|GetID_Data (Variables|Default|GetMaster_HI_reference)) (Utilities|Struct|Makes_Level_Master_Collected_Actors 0 _returnvalue_3 (Utilities|GetDisplayName _returnvalue_3) true)))
          (CallFunction|FuncPrintErrorMessage (Utilities|String|Append "Assigned ID:" (Utilities|String|ToString(Integer) _returnvalue_4)) "NewEnumerator0" (Components|GetOwner) self (Variables|Default|GetPrint))
          (Variables|Default|SetRespawnID (Utilities|Struct|Makes_RespawnData_ID (Variables|/Game/World_Management/Level_Master_HI.Level_Master_HI_C|GetCoordinates (Variables|Default|GetMaster_HI_reference)) _returnvalue_4))
          (Rendering|Debug|DrawDebugLine (Transformation|GetActorLocation (Components|GetOwner)) (Transformation|GetActorLocation (Variables|Default|GetMaster_HI_reference)) "(R=0.137837,G=1.000000,B=0.000000,A=1.000000)" 0.0 2e+01 :!label _label)
          (return)
          (else
            (bind _array_element (Utilities|Array|ForEachLoopwithBreak (Variables|/Game/World_Management/Level_Master_HI.Level_Master_HI_C|GetID_Data (Variables|Default|GetMaster_HI_reference)) :!label _label_2)
              (:LoopBody
                (if (not (!= (.ID (Utilities|Struct|Breaks_Level_Master_Collected_Actors _array_element)) (+ _id 1000)))
                  (CallFunction|FuncDrawWarningBox (Utilities|String|Append "Identical Spawn ID: " (Utilities|String|ToString(Integer) _id)) (Components|GetOwner) self)
                  (goto _label_2 Break)))
              (:Completed
                (Utilities|Array|Add (Variables|/Game/World_Management/Level_Master_HI.Level_Master_HI_C|GetID_Data (Variables|Default|GetMaster_HI_reference)) (Utilities|Struct|Makes_Level_Master_Collected_Actors (+ (Variables|Default|GetID) 1000) _returnvalue_2 (Utilities|GetDisplayName _returnvalue_2) false))
                (Variables|Default|SetRespawnID (Utilities|Struct|Makes_RespawnData_ID (Variables|/Game/World_Management/Level_Master_HI.Level_Master_HI_C|GetCoordinates (Variables|Default|GetMaster_HI_reference)) (+ (Variables|Default|GetID) 1000)))
                (goto _label)))))
        (else
          (goto _label))))
    (:Is%20Not%20Valid
      (CallFunction|FuncPrintErrorMessage "Missing Master HI Link" "NewEnumerator1" _returnvalue self true)
      (if SaveArrayToMasterNode
        (CallFunction|FuncDrawWarningBox "" _returnvalue)))))

(fn DespawnEntityFunction
  (params (InitiatedByPlayer :type Boolean) (DespawnByDamage :type Boolean) (Reverse%28Respawn%29 :type Boolean))
  (bind _returnvalue (Components|GetOwner))
  (bind _respawnable (Variables|Default|GetRespawnable))
  (bind _respawnid (Variables|Default|GetRespawnID))
  (CallFunction|FuncPrintErrorMessage "Despawning" "NewEnumerator0" (Components|GetOwner) self (Variables|Default|GetPrint))
  (CallFunction|FuncPrintErrorMessage (Utilities|String|Append "Has ID:" (Utilities|String|ToString(Integer) (.ID (Utilities|Struct|Breaks_RespawnData_ID (Variables|Default|GetRespawnID))))) "NewEnumerator0" (Components|GetOwner) self (Variables|Default|GetPrint))
  (if Reverse%28Respawn%29
    (bind _game_state (CallFunction|FuncGetGameState))
    (Default|RemovefromDespawnedEntities _game_state _respawnable _respawnid)
    (else
      (bind _game_state_2 (CallFunction|FuncGetGameState))
      (Default|AddtoDespawnedEntities _game_state_2 _respawnable _respawnid)))
  (bind _game_mode (CallFunction|FuncGetGameMode))
  (Default|SaveGame (Variables|/Game/Blueprints/NewGameMode.NewGameMode_C|Getac_SaveLoadGame _game_mode) false)
  (if Reverse%28Respawn%29
    (Variables|Default|SetSpawn true)
    (Class|AcRespawnDataInterface|EntitySpawnCall(Message) _returnvalue InitiatedByPlayer)
    (else
      (Variables|Default|SetSpawn false)
      (Class|AcRespawnDataInterface|EntityDespawnCall(Message) _returnvalue InitiatedByPlayer DespawnByDamage))))

(fn RespawnDataConstructionTempjunk
  (params (Master_HI_reference :type Level%20Master%20HI%20Object%20Reference) (Respawnable :type Boolean) (ID :type Integer))
  (Variables|Default|SetMaster_HI_reference Master_HI_reference)
  (Variables|Default|SetRespawnable Respawnable)
  (Variables|Default|SetID ID)
  (Variables|Default|SetConstructed_junk true)
  (CallFunction|CreateID false)
  (return))