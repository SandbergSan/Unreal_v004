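; ac_Loot_DebugPreview is a debug preview actor that shows three loot drop pickup widgets in the world.
; On BeginPlay it creates a W_HUD_ItemPickup for each drop, fills it with that drop's display name, item and a fixed amount, and assigns it to the matching widget component.
; Every Tick it rotates the whole actor to face player pawn 0, so the previews stay turned toward the player.
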(event EventBeginPlay
  (bind _returnvalue (UserInterface|CreateWidget "/Game/HUD/w_HUD_ItemPickup.w_HUD_ItemPickup_C"))
  (Default|SetInformationHUDItemPickup _returnvalue (Variables|Default|GetDrop1_DisplayName) 1 (Variables|Default|GetDrop1_Item))
  (UserInterface|SetWidget (Variables|Default|GetDrop1) _returnvalue)
  (bind _returnvalue_2 (UserInterface|CreateWidget "/Game/HUD/w_HUD_ItemPickup.w_HUD_ItemPickup_C"))
  (Default|SetInformationHUDItemPickup _returnvalue_2 (Variables|Default|GetDrop2_DisplayName) 2 (Variables|Default|GetDrop2_Item))
  (UserInterface|SetWidget (Variables|Default|GetDrop2) _returnvalue_2)
  (bind _returnvalue_3 (UserInterface|CreateWidget "/Game/HUD/w_HUD_ItemPickup.w_HUD_ItemPickup_C"))
  (Default|SetInformationHUDItemPickup _returnvalue_3 (Variables|Default|GetDrop3_DisplayName) 3 (Variables|Default|GetDrop3_Item))
  (UserInterface|SetWidget (Variables|Default|GetDrop3) _returnvalue_3))

(event Collision|EventActorBeginOverlap
  (params (OtherActor :type Actor%20Object%20Reference)))

(event EventTick
  (params (DeltaSeconds :type Float%20%28single-precision%29))
  (Transformation|SetActorRotation (Math|Rotator|FindLookatRotation (Transformation|GetActorLocation) (Transformation|GetActorLocation (Game|Player|GetPlayerPawn 0)))))

(fn ConstructionScript)