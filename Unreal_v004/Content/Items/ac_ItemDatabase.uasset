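; Actor component item database holding arrays of Component and Weapon entries.
; GetItemInfo switches on item type and returns the Name and Item data at the given ID in the matching array.
; A temporary weapon getter, named as possibly useful later, also returns Weapon data by ID or by optional name search.
; A failed name search logs an error and falls back to the first weapon.
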(event EventBeginPlay)

(event EventTick
  (params (DeltaSeconds :type Float%20%28single-precision%29)))

(fn GetItemInfo
  (params (Type :type enum_ItemType%20Enum :default "NewEnumerator0") (ID :type Integer))
  (bind _weapons (Variables|Default|GetWeapons))
  (bind _components (Variables|Default|GetComponents))
  (bind _output (Utilities|Array|Get(acopy) _weapons ID))
  (bind _output_2 (Utilities|Array|Get(acopy) _components ID))
  (bind (_name _item) (Utilities|Struct|Breakstruct_Item_Weapon _output))
  (bind (_name_2 _item_2) (Utilities|Struct|Breakstruct_Item_Component _output_2))
  (switch Utilities|FlowControl|Switch|Switchonenum_ItemType Type
    (:NewEnumerator0
      (return _name_2 _item_2))
    (:NewEnumerator1
      (return _name _item))))

(fn TempGetWeaponMaybeuseableinfuture
  (params (ID :type Integer) (OptionalName :type Name))
  (bind _weapons (Variables|Default|GetWeapons))
  (bind _weapons_2 (Variables|Default|GetWeapons))
  (bind _output (Utilities|Array|Get(acopy) _weapons))
  (bind _output_2 (Utilities|Array|Get(acopy) _weapons_2 ID))
  (bind (_name _item _weapon) (Utilities|Struct|Breakstruct_Item_Weapon _output_2))
  (bind (_name_2 _item_2 _weapon_2) (Utilities|Struct|Breakstruct_Item_Weapon _output))
  (bind _output_get (LocalVariables|SetSearchForName OptionalName))
  (if (Utilities|Name|NotEqual(Name) _output_get "")
    (LocalVariables|SetFoundItem (LocalVariables|GetFoundItem))
    (bind (_array_element _array_index) (Utilities|Array|ForEachLoopwithBreak (Variables|Default|GetWeapons) :!label _label)
      (:LoopBody
        (if (Utilities|Name|Equal(Name) (LocalVariables|GetSearchForName) (.Name (Utilities|Struct|Breakstruct_Item_Weapon _array_element)))
          (LocalVariables|SetFoundItem true)
          (LocalVariables|SetFoundID _array_index)
          (goto _label Break)))
      (:Completed
        (if (LocalVariables|GetFoundItem)
          (return (.Name (Utilities|Struct|Breakstruct_Item_Weapon (Utilities|Array|Get(acopy) (Variables|Default|GetWeapons) (LocalVariables|GetFoundID)))) (.Item (Utilities|Struct|Breakstruct_Item_Weapon (Utilities|Array|Get(acopy) (Variables|Default|GetWeapons) (LocalVariables|GetFoundID)))) (.Weapon (Utilities|Struct|Breakstruct_Item_Weapon (Utilities|Array|Get(acopy) (Variables|Default|GetWeapons) (LocalVariables|GetFoundID)))))
          (else
            (CallFunction|FuncPrintErrorMessage (Utilities|String|Append "No item found by the name of: " (Utilities|String|ToString(Name) (LocalVariables|GetSearchForName))) "NewEnumerator2" (Components|GetOwner) self true)
            (return _name_2 _item_2 _weapon_2)))))
    (else
      (return _name _item _weapon))))