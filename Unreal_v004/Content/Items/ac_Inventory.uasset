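; Inventory actor component, meant only for the World Master, that stores items the player picks up.
; BeginPlay caches the owning World Master, or logs an error if the owner is something else.
; AddItemToInventory sums stackable types into an Inventory map keyed by ID and type, while other types go into Backpack as single entries.
; It then looks up the item in the database component and shows a HUD pickup indicator.
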(event EventBeginPlay
  (bind _asworld_master (Utilities|Casting|CastToWorld_Master (Components|GetOwner))
    (:then
      (Variables|Default|SetWorldMaster _asworld_master))
    (:CastFailed
      (CallFunction|FuncPrintErrorMessage "The inventory component should only be in a World Master." "NewEnumerator3" (Components|GetOwner) self true))))

(event EventTick
  (params (DeltaSeconds :type Float%20%28single-precision%29)))

(fn AddItemtoInventory
  (params (InventoryAdd :type Struct%20Inventory%20Add%20Structure%20%28by%20ref%29))
  (bind (_id_name _type _amount) (Utilities|Struct|Breakstruct_InventoryAdd InventoryAdd))
  (bind _inventory (Variables|Default|GetInventory))
  (bind _inventory_2 (Variables|Default|GetInventory))
  (bind _worldmaster (Variables|Default|GetWorldMaster))
  (bind _struct_inventoryslot (Utilities|Struct|Makestruct_InventorySlot _id_name _type))
  (bind (_value _returnvalue) (Utilities|Map|Find _inventory _struct_inventoryslot))
  (LocalVariables|Setlocal_Value _amount)
  (switch Utilities|FlowControl|Switch|Switchonenum_ItemType _type
    (:NewEnumerator0
      (if _returnvalue :!label _label
        (Utilities|Map|Add _inventory_2 _struct_inventoryslot (+ _value (LocalVariables|Getlocal_Value)))
        (else
          (Utilities|Map|Add _inventory_2 _struct_inventoryslot (LocalVariables|Getlocal_Value)))))
    (:NewEnumerator1
      (LocalVariables|Setlocal_Value 1 :!label _label_2)
      (Utilities|Array|Add (Variables|Default|GetBackpack) _struct_inventoryslot))
    (:NewEnumerator2
      (goto _label))
    (:NewEnumerator3
      (goto _label_2))
    (:NewEnumerator4
      (goto _label))
    (:NewEnumerator5
      (goto _label_2))
    (:NewEnumerator6
      (goto _label_2))
    (:NewEnumerator7
      (goto _label))
    (:NewEnumerator8
      (goto _label_2))
    (:NewEnumerator9
      (goto _label_2)))
  (bind (_name _item) (Default|GetItemInfo (Variables|/Game/World_Management/World_Master.World_Master_C|Getac_ItemDatabase _worldmaster) _id_name _type))
  (Default|AddPickupIndicator (Variables|/Game/World_Management/World_Master.World_Master_C|Getw_HUD _worldmaster) _name (LocalVariables|Getlocal_Value) _item)
  (return))