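; Level loader component, marked junk: its InitiateLoading, ContinueLoading and UnloadHI events are empty, and the EventGraph logic is disconnected.
; That logic shows a loading screen, builds map names from grid coordinates, and adds "HI" variants where a box overlap finds a DefaultPawn.
; It loads maps through streaming levels or level instances, with debug reporting.
; Macros handle streaming visibility, load polling, and recording HI maps for later unloading.
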(event Custom|ContinueLoading
  (params (NewLoad :type Boolean) (Streaming :type Boolean))
  ;[0 0 0] Comment
)

(event Custom|InitiateLoading
  ;[0 0 0] Comment
)

(event Custom|UnloadHI
  ;[0 0 0] Comment
)

(event EventBeginPlay
  ;[0 0 0] Comment
)

(event EventTick
  (params (DeltaSeconds :type Float%20%28single-precision%29))
  ;[0 0 0] Comment
)