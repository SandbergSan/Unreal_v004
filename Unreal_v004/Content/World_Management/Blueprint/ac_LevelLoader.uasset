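; Level loader component that opens the world level behind a loading screen and streams in its coordinate-named grid of sublevels.
; InitiateLoading opens the world, then ContinueLoading scans the XYZ bounds, skips excluded maps, adds extra levels and restores player input.
; High-detail "HI" variants load only where a box overlap finds the player.
; A flag picks direct loading or queued loading with optional per-level flushing; only queued mode records HI levels for UnloadHI.
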(event Custom|ContinueLoading
  (params (ReportMissingLevels :type Boolean))
  ;[1 1 1 1 36] This is called after the InitiateLoading event. It will be called automaticly from the World_Master when a level that has a World_Master has been opened.
  (Variables|Default|SetReportMissingLevels ReportMissingLevels)
  (CallFunction|FuncPrintErrorMessage "Continuing Loading Levels..." "NewEnumerator0" (Components|GetOwner) self (Variables|Default|GetPrint))
  ;[1 1 1 1 78] This loops through all names determined by the LowXYZ and HighXYZ settings and checks if corresponding levels are available.
  (for _index (range (+ (Variables|Default|GetLowX) 1000) (+ (Variables|Default|GetHighX) 1000))
    (for _index_2 (range (+ (Variables|Default|GetLowY) 1000) (+ (Variables|Default|GetHighY) 1000))
      (for _index_3 (range (+ (Variables|Default|GetLowZ) 1000) (+ (Variables|Default|GetHighZ) 1000))
        (if (!= (Utilities|Array|FindItem (Variables|Default|GetDontLoadTheseLevels) (Utilities|String|Append "Map" (Utilities|String|RightChop (Utilities|String|ToString(Integer) _index) 1) (Utilities|String|RightChop (Utilities|String|ToString(Integer) _index_2) 1) (Utilities|String|RightChop (Utilities|String|ToString(Integer) _index_3) 1))) -1)
          (CallFunction|FuncPrintErrorMessage (Utilities|String|Append "Ignored to load level: " (Utilities|String|Append "Map" (Utilities|String|RightChop (Utilities|String|ToString(Integer) _index) 1) (Utilities|String|RightChop (Utilities|String|ToString(Integer) _index_2) 1) (Utilities|String|RightChop (Utilities|String|ToString(Integer) _index_3) 1))) "NewEnumerator0" (Components|GetOwner) self (Variables|Default|GetPrint))
          (else
            ;;[0 0.2192 1] Read more about the difference of these in the big blue areas below.
            (if (Variables|Default|GetTemp_LoadingV2)
              (Utilities|CheckLevelIsValid (Utilities|String|StringToName (Utilities|String|Append "Map" (Utilities|String|RightChop (Utilities|String|ToString(Integer) _index) 1) (Utilities|String|RightChop (Utilities|String|ToString(Integer) _index_2) 1) (Utilities|String|RightChop (Utilities|String|ToString(Integer) _index_3) 1))) false
                (:Found%20The%20Level
                  _))
              (else
                (Utilities|Array|Add (Variables|Default|GetLevelsToLoad) (Utilities|String|Append "Map" (Utilities|String|RightChop (Utilities|String|ToString(Integer) _index) 1) (Utilities|String|RightChop (Utilities|String|ToString(Integer) _index_2) 1) (Utilities|String|RightChop (Utilities|String|ToString(Integer) _index_3) 1)))))
            (bind (_scale_worldgrid _scale_showlevel _scale_loadlevel _scale_unloadlevel _position) (CallFunction|FuncCalcLevelPosition (Utilities|Struct|Makes_Level_Master_Coordinates (- _index 1000) (- _index_2 1000) (- _index_3 1000))))
            (bind _outactors (Collision|BoxOverlapActors _position (* _scale_loadlevel 0.5) (Utilities|Array|MakeArray "ObjectTypeQuery3") "/Game/Player/FPS_Player.FPS_Player_C" :!class /Script/Engine.KismetSystemLibrary))
            (for _array_element _outactors
              ;;[1 1 1 1 36] This loop checks if the player is within the range for the Level_Master_HIs to load its content.
              (Utilities|Casting|CastToFPS_Player _array_element
                (:then
                  ;;;[0 0.2192 1] Read more about the difference of these in the big blue areas below.
                  (if (Variables|Default|GetTemp_LoadingV2)
                    (Utilities|CheckLevelIsValid (Utilities|String|StringToName (Utilities|String|Append (Utilities|String|Append "Map" (Utilities|String|RightChop (Utilities|String|ToString(Integer) _index) 1) (Utilities|String|RightChop (Utilities|String|ToString(Integer) _index_2) 1) (Utilities|String|RightChop (Utilities|String|ToString(Integer) _index_3) 1)) "HI")) true
                      (:Found%20The%20Level
                        _))
                    (else
                      (Utilities|Array|Add (Variables|Default|GetLevelsToLoadHI) (Utilities|String|Append (Utilities|String|Append "Map" (Utilities|String|RightChop (Utilities|String|ToString(Integer) _index) 1) (Utilities|String|RightChop (Utilities|String|ToString(Integer) _index_2) 1) (Utilities|String|RightChop (Utilities|String|ToString(Integer) _index_3) 1)) "HI"))))
                  (Rendering|Debug|DrawDebugBox _position (* _scale_loadlevel 0.5) "(R=0.000000,G=1.000000,B=0.092295,A=1.000000)" "0, 0, 0" 1e+01 3e+01))
                (:CastFailed
                  (CallFunction|FuncPrintErrorMessage (Utilities|String|Append (Utilities|GetClassDisplayName (Utilities|GetClass _array_element)) " is overlappinglevelmaster, shouldnt trigger") "NewEnumerator1" _array_element self true)))))))))
  (if (Variables|Default|GetTemp_LoadingV2)
    ;[0 0.2192 1] This mode is enabled if Temp_LoadingV2 is true. It is as fast as the other mode with Temp_FlushBetweenLevelLoads_onV1 turned true, and it also has the same pros and cons. This mode is still left in in case it is a better mode once the levels have some loading times. Note that this mode does not use the UnloadTheseMapsWhenLoading array, so it does not Unload any correct HI-levels at the moment.
    (for _array_element_2 (Variables|Default|GetAdditionalLevels)
      (Utilities|CheckLevelIsValid (Utilities|String|StringToName _array_element_2) (Utilities|String|EndsWith _array_element_2 "HI" "CaseSensitive")
        (:Did%20Not%20Find%20The%20Level
          (Development|PrintString "ERROR - Did not find the level" true true "(R=1.000000,G=0.000000,B=0.007827,A=1.000000)" 4e+01))))
    (Class|GameplayStatics|FlushLevelStreaming)
    (else
      ;[0 0.2192 1] This mode is slower if Temp_FlushBetweenLevelLoads_onV1 is true, but it allows the Loading Screen to update. It might be it is just slightly slower once the levels has some loading time to speak of compared to the empty Levels that this was tried on.
      (for _array_element_3 (Variables|Default|GetAdditionalLevels)
        (if (Utilities|String|EndsWith _array_element_3 "HI" "CaseSensitive")
          (Utilities|Array|AddUnique (Variables|Default|GetLevelsToLoadHI) _array_element_3)
          (else
            (Utilities|Array|AddUnique (Variables|Default|GetLevelsToLoad) _array_element_3))))
      (Utilities|LoadLevelsfromStringArray (Variables|Default|GetLevelsToLoad) false
        (:Completed
          (Utilities|LoadLevelsfromStringArray (Variables|Default|GetLevelsToLoadHI) true
            (:Completed
              (if (Variables|Default|GetTemp_FlushBetweenLevelLoads_onV1)
                _
                (else
                  (Class|GameplayStatics|FlushLevelStreaming)))))))))
  ;[1 1 1 1 36] Reports what maps where loaded and which ones failed. This can be turned off on the World Master with the Report Missing Levels set to false.
  (if (Variables|Default|GetReportMissingLevels)
    (for _array_element_4 (Variables|Default|GetMapsThatCouldLoad)
      (CallFunction|FuncPrintErrorMessage (Utilities|String|Append "Loaded Map:" _array_element_4) "NewEnumerator0" (Components|GetOwner) self (Variables|Default|GetPrint)))
    (for _array_element_5 (Variables|Default|GetMapsThatCouldNotLoad)
      (CallFunction|FuncPrintErrorMessage (Utilities|String|Append "Could not load map: " _array_element_5) "NewEnumerator1" (Components|GetOwner) self true))
    (for _array_element_6 (Variables|Default|GetMapsThatCouldNotLoadHI)
      (CallFunction|FuncPrintErrorMessage (Utilities|String|Append "Could not load HI map: " _array_element_6) "NewEnumerator1" (Components|GetOwner) self true)))
  (CallFunction|FuncPrintErrorMessage (Utilities|String|Append "Loading Complete. Loading took: " (Utilities|String|ToString(Float) (- (Utilities|Time|GetTimeSeconds) (Variables|Default|GetTimestamp))) " seconds.") "NewEnumerator0" (Components|GetOwner) self (Variables|Default|GetPrint))
  (CallFunction|FuncSetInputCharacter (Components|GetOwner) self true)
  ;[1 1 1] Artificial Delay so that the game has time to spawn actors that arent sure if they should be visible at the very beginning of a load.
  (Utilities|FlowControl|Delay 0.5)
  (Widget|RemovefromParent (Variables|Default|GetLoadingScreen)))

(event Custom|ReloadHI
  (params (ReportMissingLevels :type Boolean))
  ;[1 1 1 1 36] This event can be used for Loading or maybe teleportation, but is unused at the moment.
  (Variables|Default|SetReportMissingLevels ReportMissingLevels)
  ;[1 1 1 1 78] This loops through all names determined by the LowXYZ and HighXYZ settings and checks if corresponding levels are available.
  (for _index (range (+ (Variables|Default|GetLowX) 1000) (+ (Variables|Default|GetHighX) 1000))
    (for _index_2 (range (+ (Variables|Default|GetLowY) 1000) (+ (Variables|Default|GetHighY) 1000))
      (for _index_3 (range (+ (Variables|Default|GetLowZ) 1000) (+ (Variables|Default|GetHighZ) 1000))
        (if (!= (Utilities|Array|FindItem (Variables|Default|GetDontLoadTheseLevels) (Utilities|String|Append "Map" (Utilities|String|RightChop (Utilities|String|ToString(Integer) _index) 1) (Utilities|String|RightChop (Utilities|String|ToString(Integer) _index_2) 1) (Utilities|String|RightChop (Utilities|String|ToString(Integer) _index_3) 1))) -1)
          (CallFunction|FuncPrintErrorMessage (Utilities|String|Append "Ignored to load level: " (Utilities|String|Append "Map" (Utilities|String|RightChop (Utilities|String|ToString(Integer) _index) 1) (Utilities|String|RightChop (Utilities|String|ToString(Integer) _index_2) 1) (Utilities|String|RightChop (Utilities|String|ToString(Integer) _index_3) 1))) "NewEnumerator0" (Components|GetOwner) self (Variables|Default|GetPrint))
          (else
            ;;[0 0.2192 1] Read more about the difference of these in the big blue areas below.
            (if (Variables|Default|GetTemp_LoadingV2)
              (Utilities|CheckLevelIsValid (Utilities|String|StringToName (Utilities|String|Append "Map" (Utilities|String|RightChop (Utilities|String|ToString(Integer) _index) 1) (Utilities|String|RightChop (Utilities|String|ToString(Integer) _index_2) 1) (Utilities|String|RightChop (Utilities|String|ToString(Integer) _index_3) 1))) false
                (:Found%20The%20Level
                  _))
              (else
                (Utilities|Array|Add (Variables|Default|GetLevelsToLoad) (Utilities|String|Append "Map" (Utilities|String|RightChop (Utilities|String|ToString(Integer) _index) 1) (Utilities|String|RightChop (Utilities|String|ToString(Integer) _index_2) 1) (Utilities|String|RightChop (Utilities|String|ToString(Integer) _index_3) 1)))))
            (bind (_scale_worldgrid _scale_showlevel _scale_loadlevel _scale_unloadlevel _position) (CallFunction|FuncCalcLevelPosition (Utilities|Struct|Makes_Level_Master_Coordinates (- _index 1000) (- _index_2 1000) (- _index_3 1000))))
            (bind _outactors (Collision|BoxOverlapActors _position (* _scale_loadlevel 0.5) (Utilities|Array|MakeArray "ObjectTypeQuery3") "/Game/Player/FPS_Player.FPS_Player_C" :!class /Script/Engine.KismetSystemLibrary))
            (for _array_element _outactors
              ;;[1 1 1 1 36] This loop checks if the player is within the range for the Level_Master_HIs to load its content.
              (Utilities|Casting|CastToFPS_Player _array_element
                (:then
                  ;;;[0 0.2192 1] Read more about the difference of these in the big blue areas below.
                  (if (Variables|Default|GetTemp_LoadingV2)
                    (Utilities|CheckLevelIsValid (Utilities|String|StringToName (Utilities|String|Append (Utilities|String|Append "Map" (Utilities|String|RightChop (Utilities|String|ToString(Integer) _index) 1) (Utilities|String|RightChop (Utilities|String|ToString(Integer) _index_2) 1) (Utilities|String|RightChop (Utilities|String|ToString(Integer) _index_3) 1)) "HI")) true
                      (:Found%20The%20Level
                        _))
                    (else
                      (Utilities|Array|Add (Variables|Default|GetLevelsToLoadHI) (Utilities|String|Append (Utilities|String|Append "Map" (Utilities|String|RightChop (Utilities|String|ToString(Integer) _index) 1) (Utilities|String|RightChop (Utilities|String|ToString(Integer) _index_2) 1) (Utilities|String|RightChop (Utilities|String|ToString(Integer) _index_3) 1)) "HI"))))
                  (Rendering|Debug|DrawDebugBox _position (* _scale_loadlevel 0.5) "(R=0.000000,G=1.000000,B=0.092295,A=1.000000)" "0, 0, 0" 1e+01 3e+01))
                (:CastFailed
                  (CallFunction|FuncPrintErrorMessage (Utilities|String|Append (Utilities|GetClassDisplayName (Utilities|GetClass _array_element)) " is overlappinglevelmaster, shouldnt trigger") "NewEnumerator1" _array_element self true)))))))))
  (if (Variables|Default|GetTemp_LoadingV2)
    ;[0 0.2192 1] This mode is enabled if Temp_LoadingV2 is true. It is as fast as the other mode with Temp_FlushBetweenLevelLoads_onV1 turned true, and it also has the same pros and cons. This mode is still left in in case it is a better mode once the levels have some loading times. Note that this mode does not use the UnloadTheseMapsWhenLoading array, so it does not Unload any correct HI-levels at the moment.
    (for _array_element_2 (Variables|Default|GetAdditionalLevels)
      (Utilities|CheckLevelIsValid (Utilities|String|StringToName _array_element_2) (Utilities|String|EndsWith _array_element_2 "HI" "CaseSensitive")
        (:Did%20Not%20Find%20The%20Level
          (Development|PrintString "ERROR - Did not find the level" true true "(R=1.000000,G=0.000000,B=0.007827,A=1.000000)" 4e+01))))
    (Class|GameplayStatics|FlushLevelStreaming)
    (else
      ;[0 0.2192 1] This mode is slower if Temp_FlushBetweenLevelLoads_onV1 is true, but it allows the Loading Screen to update. It might be it is just slightly slower once the levels has some loading time to speak of compared to the empty Levels that this was tried on.
      (for _array_element_3 (Variables|Default|GetAdditionalLevels)
        (if (Utilities|String|EndsWith _array_element_3 "HI" "CaseSensitive")
          (Utilities|Array|AddUnique (Variables|Default|GetLevelsToLoadHI) _array_element_3)
          (else
            (Utilities|Array|AddUnique (Variables|Default|GetLevelsToLoad) _array_element_3))))
      (Utilities|LoadLevelsfromStringArray (Variables|Default|GetLevelsToLoad) false
        (:Completed
          (Utilities|LoadLevelsfromStringArray (Variables|Default|GetLevelsToLoadHI) true
            (:Completed
              (if (Variables|Default|GetTemp_FlushBetweenLevelLoads_onV1)
                _
                (else
                  (Class|GameplayStatics|FlushLevelStreaming)))))))))
  ;[1 1 1 1 36] Reports what maps where loaded and which ones failed. This can be turned off on the World Master with the Report Missing Levels set to false.
  (if (Variables|Default|GetReportMissingLevels)
    (for _array_element_4 (Variables|Default|GetMapsThatCouldLoad)
      (CallFunction|FuncPrintErrorMessage (Utilities|String|Append "Loaded Map:" _array_element_4) "NewEnumerator0" (Components|GetOwner) self (Variables|Default|GetPrint)))
    (for _array_element_5 (Variables|Default|GetMapsThatCouldNotLoad)
      (CallFunction|FuncPrintErrorMessage (Utilities|String|Append "Could not load map: " _array_element_5) "NewEnumerator1" (Components|GetOwner) self true))
    (for _array_element_6 (Variables|Default|GetMapsThatCouldNotLoadHI)
      (CallFunction|FuncPrintErrorMessage (Utilities|String|Append "Could not load HI map: " _array_element_6) "NewEnumerator1" (Components|GetOwner) self true)))
  (CallFunction|FuncPrintErrorMessage (Utilities|String|Append "Loading Complete. Loading took: " (Utilities|String|ToString(Float) (- (Utilities|Time|GetTimeSeconds) (Variables|Default|GetTimestamp))) " seconds.") "NewEnumerator0" (Components|GetOwner) self (Variables|Default|GetPrint))
  (CallFunction|FuncSetInputCharacter (Components|GetOwner) self true)
  ;[1 1 1] Artificial Delay so that the game has time to spawn actors that arent sure if they should be visible at the very beginning of a load.
  (Utilities|FlowControl|Delay 0.5)
  (Widget|RemovefromParent (Variables|Default|GetLoadingScreen)))

(event Custom|InitiateLoading
  ;[1 0.748 0.02034 1 36] This is called in the current level you are in. It will Open a new level and stop executing itself once the level loading starts.
  (CallFunction|FuncPrintErrorMessage "Initiating Loading Levels..." "NewEnumerator0" (Components|GetOwner) self (Variables|Default|GetPrint))
  (Variables|Default|SetTimestamp (Utilities|Time|GetTimeSeconds))
  ;;[1 0.748 0.02034] After the Loading Screen Widget has been shown, it will remove itself once the Open Level function is called.
  (Utilities|ShowLoadingScreen
    (:Complete
      (CallFunction|FuncPrintErrorMessage (Utilities|String|Append "Opening level:" (Utilities|String|ToString(Name) (Variables|Default|GetWorldName))) "NewEnumerator0" (Components|GetOwner) self (Variables|Default|GetPrint))
      (Game|OpenLevel(byName) (Variables|Default|GetWorldName)))))

(event Custom|UnloadHI
  ;[1 1 1 1 36] This event can be used for Loading or maybe teleportation, but is unused at the moment.
  (CallFunction|FuncPrintErrorMessage "Unloading HI Levels..." "NewEnumerator0" (Components|GetOwner) self (Variables|Default|GetPrint))
  (Variables|Default|SetTimestamp (Utilities|Time|GetTimeSeconds))
  ;;[1 1 1] After the Loading Screen Widget has been shown, it will remove itself once the Open Level function is called.
  (Utilities|ShowLoadingScreen
    (:Complete
      (for _array_element (Variables|Default|GetUnloadable_HI_Levels)
        (CallFunction|FuncPrintErrorMessage (Utilities|String|Append "Unloading Map:" _array_element) "NewEnumerator0" (Components|GetOwner) self (Variables|Default|GetPrint))
        (Variables|/Script/Engine.LevelStreaming|SetbShouldBeLoaded (Class|GameplayStatics|GetStreamingLevel (Utilities|String|StringToName _array_element)) false)
        (Variables|/Script/Engine.LevelStreaming|SetbShouldBeVisible (Class|GameplayStatics|GetStreamingLevel (Utilities|String|StringToName _array_element)) false))
      (Class|GameplayStatics|FlushLevelStreaming)
      (CallFunction|FuncPrintErrorMessage "Unloading HI Levels Done..." "NewEnumerator0" (Components|GetOwner) self (Variables|Default|GetPrint)))))