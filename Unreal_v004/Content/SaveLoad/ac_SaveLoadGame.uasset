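; Actor component that saves and loads player progress in a named slot: four item containers, despawned entity IDs and the respawn transform.
; SaveLoadGame branches on IsSave to write or read an sg_MySaveGame, returning success and any loaded data.
; NewFunction0 and NewFunction1 convert inventory, stock, dropped and backpack maps to and from struct arrays.
; Item type enums are stored as numeric IDs through explicit lookup functions in both directions.
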(event EventBeginPlay)

(event EventTick
  (params (DeltaSeconds :type Float%20%28single-precision%29)))

(fn SaveLoadGame
  (params (Save_Game_Name :type String) (Is_Save :type Boolean) (Save_Inventory :type Map%20of%20Struct%20Inventory%20Slot%20Structures%20to%20Integers) (Save_Stock :type Map%20of%20Struct%20Inventory%20Slot%20Structures%20to%20Integers) (Save_Dropped :type Map%20of%20Struct%20Inventory%20Slot%20Structures%20to%20Integers) (Save_Backpack :type Map%20of%20Struct%20Inventory%20Slot%20Structures%20to%20Integers) (Save%20DespawnedEntities_Permanent_IDs :type Array%20of%20S%20Respawn%20Data%20ID%20Structures) (Save%20DespawnedEntities_Respawnable_IDs :type Array%20of%20S%20Respawn%20Data%20ID%20Structures) (SavePlayerRespawnLocation :type Vector) (SavePlayerRespawnRotation :type Float%20%28single-precision%29))
  (bind _array (Utilities|Array|MakeArray ""))
  (bind _map (Utilities|Map|MakeMap "" 0))
  (LocalVariables|Setlocal_Save_Game_Name Save_Game_Name)
  (if Is_Save
    (CallFunction|FuncPrintErrorMessage (Utilities|String|Append "Saving Game >>> " (LocalVariables|Getlocal_Save_Game_Name) "...") "NewEnumerator0" (Components|GetOwner) self (Variables|Default|GetPrint))
    (bind _returnvalue (SaveGame|CreateSaveGameObject "/Game/SaveLoad/sg_MySaveGame.sg_MySaveGame_C"))
    ;[1 1 1] Converts the inventory to a saveable form
    (bind _slotsave (CallFunction|NewFunction0 Save_Inventory))
    (Variables|/Game/SaveLoad/sg_MySaveGame.sg_MySaveGame_C|SetInventory _returnvalue _slotsave)
    (bind _slotsave_2 (CallFunction|NewFunction0 Save_Stock))
    (Variables|/Game/SaveLoad/sg_MySaveGame.sg_MySaveGame_C|SetStock _returnvalue _slotsave_2)
    (bind _slotsave_3 (CallFunction|NewFunction0 Save_Dropped))
    (Variables|/Game/SaveLoad/sg_MySaveGame.sg_MySaveGame_C|SetDropped _returnvalue _slotsave_3)
    (bind _slotsave_4 (CallFunction|NewFunction0 Save_Backpack))
    (Variables|/Game/SaveLoad/sg_MySaveGame.sg_MySaveGame_C|SetBackpack _returnvalue _slotsave_4)
    (Variables|/Game/SaveLoad/sg_MySaveGame.sg_MySaveGame_C|SetDespawnedEntities_Permanent_IDs _returnvalue Save%20DespawnedEntities_Permanent_IDs)
    (Variables|/Game/SaveLoad/sg_MySaveGame.sg_MySaveGame_C|SetDespawnedEntities_Respawnable_IDs _returnvalue Save%20DespawnedEntities_Respawnable_IDs)
    (Variables|/Game/SaveLoad/sg_MySaveGame.sg_MySaveGame_C|SetPlayerRespawnLocation _returnvalue SavePlayerRespawnLocation)
    (Variables|/Game/SaveLoad/sg_MySaveGame.sg_MySaveGame_C|SetPlayerRespawnRotation _returnvalue SavePlayerRespawnRotation)
    (bind _returnvalue_2 (SaveGame|SaveGametoSlot _returnvalue (LocalVariables|Getlocal_Save_Game_Name)))
    (return _returnvalue_2 _map _map _map _map _array _array "0, 0, 0" 0.0)
    (else
      (CallFunction|FuncPrintErrorMessage (Utilities|String|Append "Loading Game >>> " (LocalVariables|Getlocal_Save_Game_Name) "...") "NewEnumerator0" (Components|GetOwner) self (Variables|Default|GetPrint))
      (bind _returnvalue_3 (SaveGame|LoadGamefromSlot (LocalVariables|Getlocal_Save_Game_Name)))
      (bind _assg_my_save_game (Utilities|Casting|CastTosg_MySaveGame _returnvalue_3)
        (:then
          ;[1 1 1] Converts the saved inventory to a useable form.
          (bind _inventory (CallFunction|NewFunction1 (Variables|/Game/SaveLoad/sg_MySaveGame.sg_MySaveGame_C|GetInventory _assg_my_save_game)))
          (bind _inventory_2 (CallFunction|NewFunction1 (Variables|/Game/SaveLoad/sg_MySaveGame.sg_MySaveGame_C|GetStock _assg_my_save_game)))
          (bind _inventory_3 (CallFunction|NewFunction1 (Variables|/Game/SaveLoad/sg_MySaveGame.sg_MySaveGame_C|GetDropped _assg_my_save_game)))
          (bind _inventory_4 (CallFunction|NewFunction1 (Variables|/Game/SaveLoad/sg_MySaveGame.sg_MySaveGame_C|GetBackpack _assg_my_save_game)))
          (return true _inventory _inventory_2 _inventory_3 _inventory_4 (Variables|/Game/SaveLoad/sg_MySaveGame.sg_MySaveGame_C|GetDespawnedEntities_Permanent_IDs _assg_my_save_game) (Variables|/Game/SaveLoad/sg_MySaveGame.sg_MySaveGame_C|GetDespawnedEntities_Respawnable_IDs _assg_my_save_game) (Variables|/Game/SaveLoad/sg_MySaveGame.sg_MySaveGame_C|GetPlayerRespawnLocation _assg_my_save_game) (Variables|/Game/SaveLoad/sg_MySaveGame.sg_MySaveGame_C|GetPlayerRespawnRotation _assg_my_save_game)))
        (:CastFailed
          (CallFunction|FuncPrintErrorMessage "Wrong Load Game type" "NewEnumerator3" (Components|GetOwner) self true)
          (return false 0 0 0 0 0 0 "0, 0, 0" 0.0))))))

(fn GetItemTypeID
  (params (Selection :type enum_ItemType%20Enum :default "NewEnumerator0"))
  (switch Utilities|FlowControl|Switch|Switchonenum_ItemType Selection
    (:NewEnumerator0
      (return 0))
    (:NewEnumerator1
      (return 1))
    (:NewEnumerator2
      (return 2))
    (:NewEnumerator3
      (return 3))
    (:NewEnumerator4
      (return 4))
    (:NewEnumerator5
      (return 5))
    (:NewEnumerator6
      (return 6))
    (:NewEnumerator7
      (return 7))
    (:NewEnumerator8
      (return 8))
    (:NewEnumerator9
      (return 9))))

(fn GetItemTypeEnum
  (params (ID :type Byte))
  (switch int (Math|Conversions|ToInteger(Byte) ID)
    (:Default
      _)
    (:0
      _)
    (:1
      (return "NewEnumerator1"))
    (:2
      (return "NewEnumerator2"))
    (:3
      (return "NewEnumerator3"))
    (:4
      (return "NewEnumerator4"))
    (:5
      (return "NewEnumerator5"))
    (:6
      (return "NewEnumerator6"))
    (:7
      (return "NewEnumerator7"))
    (:8
      (return "NewEnumerator8"))
    (:9
      (return "NewEnumerator9")))
  (return "NewEnumerator0"))

(fn NewFunction0
  (params (Map :type Map%20of%20Struct%20Inventory%20Slot%20Structures%20to%20Integers))
  (Utilities|Array|Clear (LocalVariables|GetInventorySave))
  (bind _keys (Utilities|Map|Keys Map))
  (for (_array_element _array_index) _keys
    (bind _values (Utilities|Map|Values Map))
    (bind _typeid (CallFunction|GetItemTypeID (.Type (Utilities|Struct|Breakstruct_InventorySlot _array_element))))
    (Utilities|Array|Add (LocalVariables|GetInventorySave) (Utilities|Struct|Makestruct_InventorySlotSave (.ID_Name (Utilities|Struct|Breakstruct_InventorySlot _array_element)) _typeid (Utilities|Array|Get(acopy) _values _array_index))))
  (return (LocalVariables|GetInventorySave)))

(fn NewFunction1
  (params (Inventory_Slot_Save :type Array%20of%20Struct%20Inventory%20Slot%20Save%20Structures))
  (Utilities|Map|Clear (LocalVariables|GetMapLoad))
  (for _array_element Inventory_Slot_Save
    (bind _enum (CallFunction|GetItemTypeEnum (.TypeID (Utilities|Struct|Breakstruct_InventorySlotSave _array_element))))
    (Utilities|Map|Add (LocalVariables|GetMapLoad) (Utilities|Struct|Makestruct_InventorySlot (.ID_Name (Utilities|Struct|Breakstruct_InventorySlotSave _array_element)) _enum) (.Amount (Utilities|Struct|Breakstruct_InventorySlotSave _array_element))))
  (return (LocalVariables|GetMapLoad)))