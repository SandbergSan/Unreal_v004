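; Pawn for the startup menu that puts the menu widget on screen when play begins.
; On BeginPlay it creates StartupMenu_Widget, adds it to the viewport and switches player 0 to UI-only input focused on that widget.
; It hides the mouse cursor, waits through a short delay, then shows it again, printing debug messages along the way.
; Alternative input-mode nodes are left unconnected.
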(event EventBeginPlay
  (bind _returnvalue (Game|GetPlayerController 0))
  (bind _returnvalue_2 (UserInterface|CreateWidget "/Game/Blueprints/StartupMenu_Widget.StartupMenu_Widget_C" _returnvalue))
  (UserInterface|Viewport|AddtoViewport _returnvalue_2 0)
  (Input|SetInputModeUIOnly _returnvalue _returnvalue_2 "DoNotLock")
  (Variables|/Script/Engine.PlayerController|SetbShowMouseCursor _returnvalue false)
  (Development|PrintString "WRONG MOUSE SHOWaaaaaa" true true "(R=1.000000,G=0.046773,B=0.000000,A=1.000000)" 22.0)
  (Utilities|FlowControl|Delay 4.0)
  (Development|PrintString "Hello")
  (Variables|/Script/Engine.PlayerController|SetbShowMouseCursor _returnvalue true)
  (Development|PrintString "WRONG MOUSE SHOWffggffgj" true true "(R=1.000000,G=0.046773,B=0.000000,A=1.000000)" 22.0))

(event Collision|EventActorBeginOverlap
  (params (OtherActor :type Actor%20Object%20Reference)))

(event EventTick
  (params (DeltaSeconds :type Float%20%28single-precision%29)))

(fn ConstructionScript)