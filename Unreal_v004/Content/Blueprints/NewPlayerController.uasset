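; Player controller that handles global hotkeys for menus, saving, loading and testing.
; Each key is gated by an InputsEnabled flag, toggled through Enable_HUD_Inputs and Disable_HUD_Inputs events.
; Keys open HUD widgets, including a debug window hidden in distribution builds, or call the game mode to save, soft-load, start level loading and simulate death with a save and respawn.
; Leftover input-toggling and print test chains are unconnected.
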(event Custom|Enable_HUD_Inputs
  (Variables|Default|SetInputs_Enabled true))

(event Custom|Disable_HUD_Inputs
  (Variables|Default|SetInputs_Enabled false))

(event EventBeginPlay)

(event EventTick
  (params (DeltaSeconds :type Float%20%28single-precision%29)))

(event Input|KeyboardEvents|F7
  (params (Key :type Key%20Structure))
  (:Pressed
    (if (Variables|Default|GetInputs_Enabled)
      (bind _game_mode (CallFunction|FuncGetGameMode))
      (Default|LoadGameSoft _game_mode))))

(event Input|KeyboardEvents|I
  (params (Key :type Key%20Structure))
  (:Pressed
    (if (Variables|Default|GetInputs_Enabled)
      (bind _hud (CallFunction|FuncGetHUD))
      (Default|ShowWidget _hud "NewEnumerator0" true false))))

(event Input|KeyboardEvents|F6
  (params (Key :type Key%20Structure))
  (:Pressed
    (if (Variables|Default|GetInputs_Enabled)
      (bind _game_mode (CallFunction|FuncGetGameMode))
      (Default|SaveGame (Variables|/Game/Blueprints/NewGameMode.NewGameMode_C|Getac_SaveLoadGame _game_mode) true))))

(event Input|KeyboardEvents|L
  (params (Key :type Key%20Structure))
  (:Pressed
    (if (Variables|Default|GetInputs_Enabled)
      (bind _hud (CallFunction|FuncGetHUD))
      (Default|ShowWidget _hud "NewEnumerator5" true false))))

(event Input|KeyboardEvents|R
  (params (Key :type Key%20Structure))
  (bind _self self)
  (:Pressed
    (if (Variables|Default|GetInputs_Enabled)
      (CallFunction|FuncPrintErrorMessage "Simulate dying...." "NewEnumerator0" _self _self true)
      (bind _game_mode (CallFunction|FuncGetGameMode))
      (Default|SaveGame (Variables|/Game/Blueprints/NewGameMode.NewGameMode_C|Getac_SaveLoadGame _game_mode) true)
      (Default|RespawnPlayer (Variables|/Game/Blueprints/NewGameMode.NewGameMode_C|Getac_SaveLoadGame _game_mode)))))

(event Input|KeyboardEvents|K
  (params (Key :type Key%20Structure))
  (:Pressed
    (if (Variables|Default|GetInputs_Enabled)
      (bind _game_mode (CallFunction|FuncGetGameMode))
      (Default|InitiateLoading (Variables|/Game/Blueprints/NewGameMode.NewGameMode_C|Getac_LevelLoader _game_mode)))))

(event Input|KeyboardEvents|Subtract
  (params (Key :type Key%20Structure))
  ;[0.7563 0 1 1 36] Debug Window
  (:Pressed
    (if (Variables|Default|GetInputs_Enabled)
      (if (not (Class|KismetSystemLibrary|IsPackagedforDistribution))
        (bind _hud (CallFunction|FuncGetHUD))
        (Default|ShowWidget _hud "NewEnumerator3" true false)))))

(fn ConstructionScript)