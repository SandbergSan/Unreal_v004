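; Game mode for the startup menu that overrides BeginPlay to abort it, with no call to the parent event.
; BeginPlay casts itself to NewGameMode and logs the override through FuncPrintErrorMessage, using that class's Print setting to enable output.
; A failed cast instead reports an incorrect parent class with an explicit severity.
; Tick is disabled and the construction script only calls its parent.
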(event EventBeginPlay
  (bind _self self)
  (bind _asnew_game_mode (Utilities|Casting|CastToNewGameMode self)
    (:then
      (CallFunction|FuncPrintErrorMessage "Game Mode BeginPlay was overridden and aborted." "NewEnumerator0" self _asnew_game_mode (Variables|/Game/Blueprints/NewGameMode.NewGameMode_C|GetPrint _asnew_game_mode)))
    (:CastFailed
      (CallFunction|FuncPrintErrorMessage "Not Correct Parent Class" "NewEnumerator3" _self _self true))))

(event EventTick
  (params (DeltaSeconds :type Float%20%28single-precision%29))
  (|CallParentFunction DeltaSeconds) ; This node is disabled and will not be called.\nDrag off pins to build functionality.
)

(fn ConstructionScript
  (|CallParentFunction))