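; Game mode that runs world startup, save and load, and player respawn.
; On begin play it shows a menu widget in the whole-world level; otherwise it unloads HI levels, loads the save and continues streaming through AcLevelLoader.
; AcSaveLoadGame handles save data; loading and respawning move the player to the spawn point stored in PlayerState.
; Development builds flag duplicate Level_Master coordinates, while packaged builds override debug flags in the construction script.
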(event Custom|Save%20Game
  (bind _self self)
  (bind _success (Default|SaveLoadGame (Variables|Default|Getac_SaveLoadGame) (Variables|Default|GetSaveGameName) true))
  (if (not _success)
    (CallFunction|FuncPrintErrorMessage "Could Not Save Game" "NewEnumerator3" _self _self true)))

(event Custom|RespawnPlayer
  (Default|UnloadHI (Variables|Default|Getac_LevelLoader))
  (CallFunction|MovePlayertoSpawnSpot)
  (Default|ReloadHI (Variables|Default|Getac_LevelLoader) (Variables|Default|GetReportMissingLevels)))

(event Custom|Load%20Game
  (bind _self self)
  (bind _success (Default|SaveLoadGame (Variables|Default|Getac_SaveLoadGame) (Variables|Default|GetSaveGameName) false))
  (if _success
    (CallFunction|MovePlayertoSpawnSpot)
    (else
      (CallFunction|FuncPrintErrorMessage "Could Not Load Game" "NewEnumerator3" _self _self true))))

(event Custom|SimulatedBeginPlayOfTheOldWorldMaster_Temp
  (bind _self self)
  (Default|UnloadHI (Variables|Default|Getac_LevelLoader))
  (CallFunction|FuncPrintErrorMessage "Automatic Level Loading" "NewEnumerator0" _self _self (Variables|Default|GetPrint))
  (CallFunction|LoadGame)
  (Default|ContinueLoading (Variables|Default|Getac_LevelLoader) (Variables|Default|GetReportMissingLevels))
  (if (not (Class|KismetSystemLibrary|IsPackagedforDistribution))
    ;[0.7563 0 1] Dev Only : Just checking for duplicate Level_Masters and Level_Master_HIs. Should not be needed in Distribution since it might be slow to check. Also the delay is needed, for unknown reasons.
    (Utilities|FlowControl|Delay 2.0)
    (CallFunction|CheckforDuplicateLevelMasters)))

(event Custom|Load%20Game%20Soft
  ;[0.09896 0.09896 0.09896] probably dont use
  (Default|UnloadHI (Variables|Default|Getac_LevelLoader))
  ;;[1 0.09375 0.09375] maybe remove me, just to have time to add loading screen, but maybe not needed if fullscreen covers the movement of the player
  (Utilities|FlowControl|Delay 0.1)
  (CallFunction|LoadGame)
  (Default|ReloadHI (Variables|Default|Getac_LevelLoader) (Variables|Default|GetReportMissingLevels)))

(event Custom|Load%20Game%20Hard
  (Development|PrintString "Load Game Hard")
  (Default|InitiateLoading (Variables|Default|Getac_LevelLoader))
  (Development|PrintString "Load Game Hard DONE"))

(event EventBeginPlay
  (bind _self self)
  (bind _self_2 self)
  (bind _wholeworldname (Variables|Default|GetWholeWorldName))
  (CallFunction|FuncSetInputAllOff _self_2 _self_2 true)
  (bind _returnvalue (Game|GetCurrentLevelName true))
  (if (Utilities|Enum|Equal(Enum) _returnvalue _wholeworldname)
    (bind _hud (CallFunction|FuncGetHUD))
    (Default|ShowWidget _hud "NewEnumerator5" true true)
    (else
      (CallFunction|FuncPrintErrorMessage (Utilities|String|Append "Show Load Save Menu Aborted (Since the percistant level isn't called: " _wholeworldname ")") "NewEnumerator0" 0 0 (Variables|Default|GetPrint))
      (Default|UnloadHI (Variables|Default|Getac_LevelLoader))
      (CallFunction|FuncPrintErrorMessage "Automatic Level Loading" "NewEnumerator0" _self _self (Variables|Default|GetPrint))
      (CallFunction|LoadGame)
      (Default|ContinueLoading (Variables|Default|Getac_LevelLoader) (Variables|Default|GetReportMissingLevels))
      (if (not (Class|KismetSystemLibrary|IsPackagedforDistribution))
        ;[0.7563 0 1] Dev Only : Just checking for duplicate Level_Masters and Level_Master_HIs. Should not be needed in Distribution since it might be slow to check. Also the delay is needed, for unknown reasons.
        (Utilities|FlowControl|Delay 2.0)
        (CallFunction|CheckforDuplicateLevelMasters)))))

(event EventTick
  (params (DeltaSeconds :type Float%20%28single-precision%29)))

(fn ConstructionScript
  ;[1 1 1 1 36] Forces all debug settings to turn off when packaging for distribution.
  (if (Class|KismetSystemLibrary|IsPackagedforDistribution)
    (Variables|Default|SetReportMissingLevels true)
    (Variables|Default|SetGod_Movement false)
    (Variables|Default|SetShowItemDropsOnEntities false)
    (Variables|Default|SetPrint false)))

(fn MovePlayertoSpawnSpot
  (bind _returnvalue (Game|GetPlayerController 0))
  (bind _self self)
  (CallFunction|FuncPrintErrorMessage "Someitmes i get errors pointing here, something with get player pawn" "NewEnumerator1" _self _self (Variables|Default|GetPrint))
  (Input|DisableInput _returnvalue 0)
  (bind _asfps_player (Utilities|Casting|CastToFPS_Player (Pawn|GetControlledPawn _returnvalue)))
  (Default|DisablePawnInputs _asfps_player)
  (Pawn|Components|CharacterMovement|DisableMovement (Variables|/Script/Engine.Character|GetCharacterMovement (Game|GetPlayerCharacter 0)))
  (bind _player_state (CallFunction|FuncGetPlayerState))
  (Transformation|SetActorLocation (Game|Player|GetPlayerPawn 0) (Variables|/Game/Blueprints/NewPlayerState.NewPlayerState_C|GetPlayerRespawnLocation _player_state) false false)
  (Pawn|SetControlRotation (Game|GetPlayerController 0) (Math|Rotator|MakeRotator 0.0 0.0 (Variables|/Game/Blueprints/NewPlayerState.NewPlayerState_C|GetPlayerRespawnRotation _player_state))))

(fn CheckforDuplicateLevelMasters
  (Utilities|FlowControl|Sequence
    (:then_0
      (Utilities|Array|Clear (LocalVariables|GetUniqueCoords))
      (bind _outactors (Actor|GetAllActorsOfClass "/Game/World_Management/Level_Master.Level_Master_C"))
      (for _array_element _outactors
        (bind _returnvalue (Utilities|Array|AddUnique (LocalVariables|GetUniqueCoords) (Variables|/Game/World_Management/Level_Master.Level_Master_C|GetCoordinates _array_element)))
        (if (== _returnvalue -1)
          (CallFunction|FuncDrawWarningBox "This Level_Master has identical Coordinates as some other LevelMaster." _array_element self))))
    (:then_1
      (Utilities|Array|Clear (LocalVariables|GetUniqueCoords))
      (bind _outactors_2 (Actor|GetAllActorsOfClass "/Game/World_Management/Level_Master_HI.Level_Master_HI_C"))
      (for _array_element_2 _outactors_2
        (bind _returnvalue_2 (Utilities|Array|AddUnique (LocalVariables|GetUniqueCoords) (Variables|/Game/World_Management/Level_Master_HI.Level_Master_HI_C|GetCoordinates _array_element_2)))
        (if (== _returnvalue_2 -1)
          (CallFunction|FuncDrawWarningBox "This Level_Master_HI has identical Coordinates as some other LevelMaster_HI." _array_element_2 self))))))