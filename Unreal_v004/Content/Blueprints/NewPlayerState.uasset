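; Player state Blueprint that handles the penalty for a player who was not safe when they saved and exited.
; UpdateDropPoint checks PlayerIsSafe; if false, it logs an error, transfers inventory items between maps and records PlayerDropPoint as the drop location.
; When dropped items exist, it moves the existing IA_DropPoint actor there or spawns one, then marks the player safe.
; The event graph has no active logic.
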(event EventBeginPlay)

(event EventTick
  (params (DeltaSeconds :type Float%20%28single-precision%29)))

(fn ConstructionScript)

(fn UpdateDropPoint
  (bind _self self)
  (if (Variables|Saved|GetPlayerIsSafe)
    (Development|PrintString "PLAYER WAS SAFE")
    (else
      (CallFunction|FuncPrintErrorMessage "PLAYER WAS NOT SAFE WHEN SAVED AND EXITED" "NewEnumerator0" _self _self true)
      (bind _ac_inventory (CallFunction|FuncGetInventory))
      (Default|TransferItemsBetweenMaps _ac_inventory "NewEnumerator1")
      (Variables|Saved|SetPlayerHasDroppedItemsAt (Variables|Saved|GetPlayerDropPoint))
      (Variables|Saved|SetPlayerHasDroppedItems true)))
  (if (Variables|Saved|GetPlayerHasDroppedItems)
    (Utilities|IsValid (Variables|Default|GetDropPoint)
      (:Is%20Valid
        (Development|PrintString "MOVED ALREADY CREATED")
        (Transformation|SetActorTransform (Variables|Default|GetDropPoint) (Math|Transform|MakeTransform (Variables|Saved|GetPlayerHasDroppedItemsAt) "0, 0, 0" "1.000000,1,1.000000")))
      (:Is%20Not%20Valid
        (Development|PrintString "CREATED AND MOVED")
        (bind _returnvalue (Game|SpawnActorfromClass "/Game/Interactable_Actor/IA_DropPoint.IA_DropPoint_C" (Math|Transform|MakeTransform (Variables|Saved|GetPlayerHasDroppedItemsAt) "0, 0, 0" "1.000000,1,1.000000") "Undefined" 0 0))
        (Variables|Default|SetDropPoint _returnvalue))))
  (Variables|Saved|SetPlayerIsSafe true)
  (return))